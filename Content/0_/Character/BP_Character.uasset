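; First-person character Blueprint that takes touch input and starts play holding a default weapon.
; Thumbstick and jump touch events forward to move, aim and jump functions.
; On BeginPlay, the authority spawns the weapon with itself as owner and instigator, attaches it to the first-person mesh's right-hand socket and equips it.
; HasWeapon stores the attach result; its OnRep handler is empty.
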(event `self.Primary Thumbstick`
  (params (Axis :type "Vector2D Structure"))
  ; Touch Inputs for First Person Character
  (`self.DoMove` Axis_X Axis_Y))

(event `self.Secondary Thumbstick`
  (params (Axis :type "Vector2D Structure"))
  ; Touch Inputs for First Person Character
  (`self.DoAim` Axis_X Axis_Y))

(event `self.Touch Jump Start`
  ; Touch Inputs for First Person Character
  (`self.DoJumpStart`))

(event `self.Touch Jump End`
  ; Touch Inputs for First Person Character
  (`self.DoJumpEnd`))

(event `self.ReceiveBeginPlay`
  (`/Engine/EditorBlueprintResources/ActorMacros.Switch Has Authority`
    (:`Authority`
      (bind _returnvalue (`|SpawnActorFromClass` (`self.DefaultWeapon`) (`self.GetTransform`) "Undefined" "MultiplyWithRoot" self self))
      (cast `/Game/0_/Weapons/BP_WeaponBase` _returnvalue
        (:`then`
          (bind _output_get (set `self.CurrentWeapon` _returnvalue)))
        (:`CastFailed`
          _))
      (bind _returnvalue_2 (`self.K2_AttachToComponent` _output_get (`self.FirstPersonMesh`) "HandGrip_R" "SnapToTarget" "SnapToTarget" "KeepWorld" true))
      (set `self.hasWeapon` _returnvalue_2)
      (`self.EquipCombatWeapon` (`self.CurrentWeapon`)))))

(fn `OnRep_hasWeapon`)

(fn `UserConstructionScript`)